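; BP_SlingshotRock is the rock for an enemy slingshot ability, with logic that makes it tumble visually.
; On BeginPlay it picks independent random pitch, roll and yaw rotation rates, allowing spin in either direction.
; Each Tick applies those rates, scaled by delta time, as local rotation on RockMesh.
; The graphs shown contain no movement, collision or damage logic.
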(event EventBeginPlay
  (bind _returnvalue (Math|Random|RandomFloatinRange -5e+02 5e+02))
  (Utilities|FlowControl|Sequence
    (:then_0
      (Variables|Default|SetPitchRotationRate _returnvalue))
    (:then_1
      (Variables|Default|SetRollRotationRate _returnvalue))
    (:then_2
      (Variables|Default|SetYawRotationRate _returnvalue))))

(event EventTick
  (params (DeltaSeconds :type Float%20%28single-precision%29))
  (Transformation|AddLocalRotation (Variables|Default|GetRockMesh) (Math|Rotator|MakeRotator (* (Variables|Default|GetRollRotationRate) DeltaSeconds) (* (Variables|Default|GetPitchRotationRate) DeltaSeconds) (* (Variables|Default|GetYawRotationRate) DeltaSeconds)) false false))

(fn ConstructionScript)